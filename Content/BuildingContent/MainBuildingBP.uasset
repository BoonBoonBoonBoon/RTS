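; MainBuildingBP is a building Blueprint, apparently a base for buildings with selection widgets such as a marketplace and barracks.
; On BeginPlay it creates a BP_BuildingWidget, stores the reference and passes itself to the widget as BuildingRef.
; The open events are stubs: marketplace is empty and barracks only prints debug text.
; Logic to show, hide or remove the widget is disconnected, so this Blueprint never displays it.
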(event EventBeginPlay
  (Utilities|FlowControl|Sequence
    (:then_0
      ;[1 1 1] Create Building Selected Widget
      (bind _returnvalue (UserInterface|CreateWidget "/Game/UserContent/UserControl/Widgets/UI/BuildingUI/Marketplace/BP_BuildingWidget.BP_BuildingWidget_C"))
      (Variables|Default|SetWidgetRefrence _returnvalue)
      (Variables|/Game/UserContent/UserControl/Widgets/UI/BuildingUI/Marketplace/BP_BuildingWidget.BP_BuildingWidget_C|SetBuildingRef _returnvalue self))))

(event Collision|EventActorBeginOverlap
  (params (OtherActor :type Actor%20Object%20Reference)))

(event EventTick
  (params (DeltaSeconds :type Float%20%28single-precision%29)))

(event EventOpenBarracksWidget
  (Development|PrintText "Added"))

(event EventOpenMarketPlaceWidget)

(fn ConstructionScript)