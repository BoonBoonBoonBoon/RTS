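; Light infantry enemy AI that wanders at random and moves toward other AI pawns it spots.
; BeginPlay starts a roam loop that picks reachable points near the actor and repeats on each successful move.
; Pawn sensing accepts only GenericBaseAI pawns, sets a seen flag that is never cleared here and issues a move to the target.
; Roaming restarts if the target's IsDest is set; no damage is dealt and the attack-range overlap is empty.
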(event OnComponentBeginOverlap(AttackRangeSphere)
  (params (OverlappedComponent :type Primitive%20Component%20Object%20Reference) (OtherActor :type Actor%20Object%20Reference) (OtherComp :type Primitive%20Component%20Object%20Reference) (OtherBodyIndex :type Integer) (bFromSweep :type Boolean) (SweepResult :type Hit%20Result%20Structure%20%28by%20ref%29)))

(event OnSeePawn(PawnSensing)
  (params (Pawn :type Pawn%20Object%20Reference))
  ;[1 1 1] Attack Enemy
  (bind _asgeneric_base_ai (Utilities|Casting|CastToGenericBaseAI Pawn))
  (Variables|Default|SetAs%20Generic%20Base%20AI _asgeneric_base_ai)
  (Variables|Default|SetIsSeeingPawn true)
  (CallFunction|AttackEnemy))

(event Custom|AttackEnemy
  ;[1 1 1] Attack Enemy
  (if (Variables|Default|GetIsSeeingPawn)
    (Utilities|IsValid (Variables|Default|GetAs%20Generic%20Base%20AI)
      (:Is%20Valid
        (AI|AIMoveTo self "0, 0, 0" (stale OnSeePawn(PawnSensing) Pawn) 2e+01 false
          (:then
            _)
          (:OnSuccess
            _)
          (:OnFail
            _))
        (if (Variables|/Script/RTS.GenericBaseAI|GetIsDest (Variables|Default|GetAs%20Generic%20Base%20AI))
          (CallFunction|RandomRoam))))))

(event Custom|Random%20Roam
  (AI|AIMoveTo self (.RandomLocation (AI|Navigation|GetRandomReachablePointinRadius (Transformation|GetActorLocation) 1e+03 0 0)) 0 5.0 false
    (:OnSuccess
      (CallFunction|RandomRoam))))

(event EventBeginPlay
  (CallFunction|RandomRoam))

(fn ConstructionScript)