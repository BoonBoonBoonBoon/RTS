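; HUD blueprint that draws the translucent blue marquee rectangle for the selection tool.
; On BeginPlay it casts player controller 0 to UserController and stores the reference.
; Each DrawHUD, while that controller's CursorMoved flag is set, it draws a rect from the initial mouse position to the new one, using values the controller supplies.
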(event EventBeginPlay
  (bind _asuser_controller (Utilities|Casting|CastToUserController (Game|GetPlayerController 0)))
  (Variables|Default|SetAs%20User%20Controller _asuser_controller))

(event Collision|EventActorBeginOverlap
  (params (OtherActor :type Actor%20Object%20Reference)))

(event EventDrawHUD
  (params (SizeX :type Integer) (SizeY :type Integer))
  (bind _as_user_controller (Variables|Default|GetAs%20User%20Controller))
  (bind _as_user_controller_2 (Variables|Default|GetAs%20User%20Controller))
  (bind _initialmouseposition (Variables|/Script/RTS.UserController|GetInitialMousePosition _as_user_controller))
  (bind _newmouseposition (Variables|/Script/RTS.UserController|GetNewMousePosition _as_user_controller_2))
  (if (Variables|/Script/RTS.UserController|GetCursorMoved (Variables|Default|GetAs%20User%20Controller))
    (HUD|DrawRect "(R=0.000000,G=0.426591,B=0.927083,A=0.208000)" (.x _initialmouseposition) (.y _initialmouseposition) (- (.x _newmouseposition) (.x _initialmouseposition)) (- (.y _newmouseposition) (.y _initialmouseposition)))))

(fn ConstructionScript)